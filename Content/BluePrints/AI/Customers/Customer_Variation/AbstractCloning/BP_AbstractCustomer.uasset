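; BP_AbstractCustomer is a customer character blueprint that assembles a visual look and shows an infection effect.
; The construction script attaches Hair to the Mesh's head socket.
; PutClothon makes Outfit follow the Mesh's pose through master pose component.
; OnInfected makes the InfectionPS component visible and sets it paused.
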(event `self.OnInfected`
  (params (Cond :type Boolean))
  (`NiagaraComponent.SetPaused` (`self.InfectionPS`) true)
  (`SceneComponent.SetVisibility` (`self.InfectionPS`) true false))

(event `self.PutClothOn`
  (`SkinnedMeshComponent.SetLeaderPoseComponent` (`self.Outfit`) (`self.Mesh`) false))

(fn `UserConstructionScript`
  (`SceneComponent.K2_AttachToComponent` (`self.Hair`) (`self.Mesh`) "head" "KeepRelative" "KeepRelative" "KeepRelative" true))