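; Child customer AI variant that randomizes its look and shows infection and "craziness" particle effects.
; BeginPlay picks skin, hair and one of three outfits with materials from BP_GameManager pools, pose-linking the outfit to the body and showing a mask if CustomerComponent has one.
; It registers the sighting with the player.
; A looping timer turns the UIChild widget toward the camera; the widget is scaled to zero once enough children have been seen.
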(event `self.ReceiveBeginPlay`
  (bind _maskmesh (`self.MaskMesh`))
  (`NiagaraComponent.SetPaused` (`self.Niagara`) true)
  (`NiagaraComponent.SetPaused` (`self.InfectionPS`) true)
  (`self.FeedBackEvent`)
  (`KismetSystemLibrary.K2_SetTimer` null "UiTick" 0.001 true)
  (bind _asbp_game_manager (cast `/Game/BluePrints/Managers/BP_GameManager` (`GameplayStatics.GetGameInstance`))
    (:`then`
      (set `self.GameManagerRef` _asbp_game_manager)
      (bind _asbp_player_character (cast `/Game/BluePrints/Character/BP_PlayerCharacter` (`GameplayStatics.GetPlayerPawn` 0))
        (:`then`
          (bind _output_get (set `self.PlayerReference` _asbp_player_character))
          (`/Game/BluePrints/Character/BP_PlayerCharacter.SeeChild` _output_get)
          (`SceneComponent.K2_AttachToComponent` (`self.MaskMesh`) (`self.Mesh`) "head" "KeepWorld" "KeepWorld" "KeepWorld" true)
          (if (`CustomerComponent.HasMask` (`self.CustomerComponent`))
            (`SceneComponent.SetVisibility` _maskmesh true false)
            (else
              (`SceneComponent.SetVisibility` _maskmesh false false)))
          (`PrimitiveComponent.SetMaterial` (`self.Mesh`) 0 (`KismetArrayLibrary.Array_Random` (`/Game/BluePrints/Managers/BP_GameManager.M_CustomerSkin` (`self.GameManagerRef`))))
          (bind _output_get_2 (set `self.HairSelection` (`KismetMathLibrary.RandomIntegerInRange` 0 1)))
          (`StaticMeshComponent.SetStaticMesh` (`self.Hair`) (select `int` _output_get_2 :`0` "/Game/Assets/Character/Hair/ShortHair.ShortHair" :`1` "/Game/Assets/Character/Hair/LongHair.LongHair" :!type "StaticMesh Object Reference"))
          (`SceneComponent.K2_AttachToComponent` (`self.Hair`) (`self.Mesh`) "head" "KeepRelative" "KeepRelative" "KeepRelative" true)
          (switch `int` _output_get_2
            (:`0`
              (`PrimitiveComponent.SetMaterial` (`self.Hair`) 0 (`KismetArrayLibrary.Array_Random` (`/Game/BluePrints/Managers/BP_GameManager.M_LongHairColors` (`self.GameManagerRef`)))))
            (:`1`
              (`PrimitiveComponent.SetMaterial` (`self.Hair`) 0 (`KismetArrayLibrary.Array_Random` (`/Game/BluePrints/Managers/BP_GameManager.M_ShortHairColors` (`self.GameManagerRef`))))))
          (bind _output_get_3 (`self.SetClothes`))
          (switch `int` _output_get_3
            (:`0`
              (`PrimitiveComponent.SetMaterial` (`self.Outfit`) 0 (`KismetArrayLibrary.Array_Random` (`/Game/BluePrints/Managers/BP_GameManager.M_PoloPants0` (`self.GameManagerRef`))))
              (`PrimitiveComponent.SetMaterial` (`self.Outfit`) 1 (`KismetArrayLibrary.Array_Random` (`/Game/BluePrints/Managers/BP_GameManager.M_PoloTop1` (`self.GameManagerRef`)))))
            (:`1`
              (`PrimitiveComponent.SetMaterial` (`self.Outfit`) 0 (`KismetArrayLibrary.Array_Random` (`/Game/BluePrints/Managers/BP_GameManager.M_GirlOutFitSkirt0` (`self.GameManagerRef`))))
              (`PrimitiveComponent.SetMaterial` (`self.Outfit`) 1 (`KismetArrayLibrary.Array_Random` (`/Game/BluePrints/Managers/BP_GameManager.M_GirlOutFitShirt1` (`self.GameManagerRef`))))
              (`PrimitiveComponent.SetMaterial` (`self.Outfit`) 2 (`KismetArrayLibrary.Array_Random` (`/Game/BluePrints/Managers/BP_GameManager.M_GirlOutFitScarf2` (`self.GameManagerRef`)))))
            (:`2`
              (`PrimitiveComponent.SetMaterial` (`self.Outfit`) 0 (`KismetArrayLibrary.Array_Random` (`/Game/BluePrints/Managers/BP_GameManager.M_DungareeDungaree0` (`self.GameManagerRef`))))
              (`PrimitiveComponent.SetMaterial` (`self.Outfit`) 1 (`KismetArrayLibrary.Array_Random` (`/Game/BluePrints/Managers/BP_GameManager.M_DungareeTshirt1` (`self.GameManagerRef`)))))))
        (:`CastFailed`
          (`KismetSystemLibrary.PrintString` "Cast failed" true true (struct :`R` 1.0 :`B` 0.381343 :`A` 1.0) 5.0 :!label _label))))
    (:`CastFailed`
      (goto _label))))

(event `self.OnInfected`
  (params (Cond :type Boolean))
  (`NiagaraComponent.SetPaused` (`self.InfectionPS`) (not Cond))
  (`SceneComponent.SetVisibility` (`self.InfectionPS`) true false))

(event `self.OnLanded`
  (params (Hit :type "HitResult Structure (by ref)"))
  (`SceneComponent.SetVisibility` (`self.UIChild`) false false))

(event `UiTick`
  (bind _uichild (`self.UIChild`))
  (bind _uichild_2 (`self.UIChild`))
  (`SceneComponent.K2_SetWorldRotation` _uichild (`KismetMathLibrary.FindLookAtRotation` (`SceneComponent.K2_GetComponentLocation` _uichild) (`self.K2_GetActorLocation` (`PlayerController.PlayerCameraManager` (`GameplayStatics.GetPlayerController` 0)))) false true)
  (`SceneComponent.SetVisibility` _uichild_2 true true)
  (`Widget.SetVisibility` (`WidgetComponent.GetWidget` _uichild_2) "Visible"))

(event `FeedBackEvent`
  (bind _uichild (`self.UIChild`))
  (`KismetSystemLibrary.K2_SetTimer` null "UiTick" 0.01 true)
  (bind _asbp_player_character (cast `/Game/BluePrints/Character/BP_PlayerCharacter` (`GameplayStatics.GetPlayerPawn` 0)))
  (if (not (< (`/Game/BluePrints/Character/BP_PlayerCharacter.ChildrenSeen` _asbp_player_character) 5))
    (`SceneComponent.SetWorldScale3D` _uichild (0.0 0.0 0.0))
    (`Widget.SetRenderScale` (`WidgetComponent.GetWidget` _uichild) (0.0 0.0))))

(event `self.OnChildCraziness`
  (params (cond :type Boolean))
  (bind _niagara (`self.Niagara`))
  (if cond
    (`NiagaraComponent.SetPaused` _niagara false)
    (else
      (`NiagaraComponent.SetPaused` _niagara true))))

(fn `SetClothes`
  (returns (Output_Get :type Integer))
  (locals (ChosenClothes :type Integer))
  (bind _output_get (set `local.ChosenClothes` (`KismetMathLibrary.RandomIntegerInRange` 0 2)))
  (`SkinnedMeshComponent.SetSkinnedAssetAndUpdate` (`self.Outfit`) (select `int` _output_get :`0` "/Game/Assets/Character/Clothing/CustomerOutfits/PoloOutfit/PoloOutfit.PoloOutfit" :`1` "/Game/Assets/Character/Clothing/CustomerOutfits/GirlOutfit/SchoolOutfit02.SchoolOutfit02" :`2` "/Game/Assets/Character/Clothing/CustomerOutfits/HByxor/HByxorOutfit.HByxorOutfit" :!type "SkeletalMesh Object Reference") true)
  (`SkinnedMeshComponent.SetLeaderPoseComponent` (`self.Outfit`) (`self.Mesh`) false)
  (return _output_get))

(fn `UserConstructionScript`)