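; Mask-wearer AI customer that spawns with a randomized look and shows its mask and infection state.
; BeginPlay picks hair, one of three outfits following the body mesh via master pose, and random materials from BP_GameManager's arrays.
; CustomerComponent sets initial mask visibility; mask events toggle it and scale the no-mask icon through a reversible timeline.
; OnInfected drives the infection particles, and OnTickBroken turns the icon toward the player camera.
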(event `self.OnTickBroken`
  (bind _uinomask (`self.UINomask`))
  (`SceneComponent.K2_SetWorldRotation` _uinomask (`KismetMathLibrary.FindLookAtRotation` (`SceneComponent.K2_GetComponentLocation` _uinomask) (`self.K2_GetActorLocation` (`PlayerController.PlayerCameraManager` (`GameplayStatics.GetPlayerController` 0)))) false true))

(event `self.OnPutMask`
  (`SceneComponent.SetVisibility` (`self.MaskMesh`) true false)
  (bind (_direction _opacity_curve _newtrack_0) (`Timeline|Timeline_1` :!label _label)
    (:`Update`
      (`SceneComponent.SetWorldScale3D` (`self.UINomask`) (`KismetMathLibrary.MakeVector` _newtrack_0 _newtrack_0 _newtrack_0)))))

(event `self.OnTakeOffMask`
  (`SceneComponent.SetVisibility` (`self.MaskMesh`) false false)
  (goto _label :!via `Reverse`))

(event `self.OnInfected`
  (params (Cond :type Boolean))
  (`NiagaraComponent.SetPaused` (`self.InfectionPS`) (not Cond))
  (`SceneComponent.SetVisibility` (`self.InfectionPS`) true false))

(event `self.ReceiveBeginPlay`
  (bind _maskmesh (`self.MaskMesh`))
  (`NiagaraComponent.SetPaused` (`self.InfectionPS`) true)
  (bind _asbp_game_manager (cast `/Game/BluePrints/Managers/BP_GameManager` (`GameplayStatics.GetGameInstance`)))
  (set `self.GameManagerRef` _asbp_game_manager)
  (`PrimitiveComponent.SetMaterial` (`self.Mesh`) 0 (`KismetArrayLibrary.Array_Random` (`/Game/BluePrints/Managers/BP_GameManager.M_CustomerSkin` (`self.GameManagerRef`))))
  (`SceneComponent.K2_AttachToComponent` (`self.MaskMesh`) (`self.Mesh`) "head" "KeepWorld" "KeepWorld" "KeepWorld" true)
  (if (`CustomerComponent.HasMask` (`self.CustomerComponent`))
    (`SceneComponent.SetVisibility` _maskmesh true false)
    (`SceneComponent.SetWorldScale3D` (`self.UINomask`) (0.0 0.0 0.0))
    (else
      (`SceneComponent.SetVisibility` _maskmesh false false)))
  (bind _output_get (set `self.HairSelection` (`KismetMathLibrary.RandomIntegerInRange` 0 1)))
  (`StaticMeshComponent.SetStaticMesh` (`self.Hair`) (select `int` _output_get :`0` "/Game/Assets/Character/Hair/ShortHair.ShortHair" :`1` "/Game/Assets/Character/Hair/LongHair.LongHair" :!type "StaticMesh Object Reference"))
  (`SceneComponent.K2_AttachToComponent` (`self.Hair`) (`self.Mesh`) "head" "KeepRelative" "KeepRelative" "KeepRelative" true)
  (switch `int` _output_get
    (:`0`
      (`PrimitiveComponent.SetMaterial` (`self.Hair`) 0 (`KismetArrayLibrary.Array_Random` (`/Game/BluePrints/Managers/BP_GameManager.M_LongHairColors` (`self.GameManagerRef`)))))
    (:`1`
      (`PrimitiveComponent.SetMaterial` (`self.Hair`) 0 (`KismetArrayLibrary.Array_Random` (`/Game/BluePrints/Managers/BP_GameManager.M_ShortHairColors` (`self.GameManagerRef`))))))
  (bind _output_get_2 (`self.SetClothes`))
  (switch `int` _output_get_2
    (:`0`
      (`PrimitiveComponent.SetMaterial` (`self.Outfit`) 0 (`KismetArrayLibrary.Array_Random` (`/Game/BluePrints/Managers/BP_GameManager.M_PoloPants0` (`self.GameManagerRef`))))
      (`PrimitiveComponent.SetMaterial` (`self.Outfit`) 1 (`KismetArrayLibrary.Array_Random` (`/Game/BluePrints/Managers/BP_GameManager.M_PoloTop1` (`self.GameManagerRef`)))))
    (:`1`
      (`PrimitiveComponent.SetMaterial` (`self.Outfit`) 0 (`KismetArrayLibrary.Array_Random` (`/Game/BluePrints/Managers/BP_GameManager.M_GirlOutFitSkirt0` (`self.GameManagerRef`))))
      (`PrimitiveComponent.SetMaterial` (`self.Outfit`) 1 (`KismetArrayLibrary.Array_Random` (`/Game/BluePrints/Managers/BP_GameManager.M_GirlOutFitShirt1` (`self.GameManagerRef`))))
      (`PrimitiveComponent.SetMaterial` (`self.Outfit`) 2 (`KismetArrayLibrary.Array_Random` (`/Game/BluePrints/Managers/BP_GameManager.M_GirlOutFitScarf2` (`self.GameManagerRef`)))))
    (:`2`
      (`PrimitiveComponent.SetMaterial` (`self.Outfit`) 0 (`KismetArrayLibrary.Array_Random` (`/Game/BluePrints/Managers/BP_GameManager.M_DungareeDungaree0` (`self.GameManagerRef`))))
      (`PrimitiveComponent.SetMaterial` (`self.Outfit`) 1 (`KismetArrayLibrary.Array_Random` (`/Game/BluePrints/Managers/BP_GameManager.M_DungareeTshirt1` (`self.GameManagerRef`)))))))

(fn `SetClothes`
  (returns (Output_Get :type Integer))
  (locals (ChosenClothes :type Integer :default 0))
  (bind _output_get (set `local.ChosenClothes` (`KismetMathLibrary.RandomIntegerInRange` 0 2)))
  (`SkinnedMeshComponent.SetSkinnedAssetAndUpdate` (`self.Outfit`) (select `int` _output_get :`0` "/Game/Assets/Character/Clothing/CustomerOutfits/PoloOutfit/PoloOutfit.PoloOutfit" :`1` "/Game/Assets/Character/Clothing/CustomerOutfits/GirlOutfit/SchoolOutfit02.SchoolOutfit02" :`2` "/Game/Assets/Character/Clothing/CustomerOutfits/HByxor/HByxorOutfit.HByxorOutfit" :!type "SkeletalMesh Object Reference") true)
  (`SkinnedMeshComponent.SetLeaderPoseComponent` (`self.Outfit`) (`self.Mesh`) false)
  (return _output_get))

(fn `UserConstructionScript`)