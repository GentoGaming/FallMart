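; Anti-masker customer AI variant with a randomized look, a toggleable face mask, an infection particle effect and an overhead icon.
; BeginPlay randomizes skin, hair and outfit from GameManager material pools, with outfits following the body mesh via master pose.
; Mask events toggle the mask and scale the icons through a timeline.
; A looping timer alternates customer and mouse-hint icons until the player has slapped more than five customers.
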(event `self.OnTickBroken`
  (bind _uicustomer (`self.UICustomer`))
  (`SceneComponent.K2_SetWorldRotation` _uicustomer (`KismetMathLibrary.FindLookAtRotation` (`SceneComponent.K2_GetComponentLocation` _uicustomer) (`self.K2_GetActorLocation` (`PlayerController.PlayerCameraManager` (`GameplayStatics.GetPlayerController` 0)))) false true)
  (`SceneComponent.K2_SetWorldRotation` (`self.UIMouse1`) (`KismetMathLibrary.FindLookAtRotation` (`SceneComponent.K2_GetComponentLocation` _uicustomer) (`self.K2_GetActorLocation` (`PlayerController.PlayerCameraManager` (`GameplayStatics.GetPlayerController` 0)))) false true))

(event `self.OnPutMask`
  (`SceneComponent.SetVisibility` (`self.MaskMesh`) true false)
  (bind (_direction _opacity_curve _newtrack_0) (`Timeline|Timeline_0` :!label _label)
    (:`Update`
      (`SceneComponent.SetWorldScale3D` (`self.UICustomer`) (`KismetMathLibrary.MakeVector` _newtrack_0 _newtrack_0 _newtrack_0))
      (`SceneComponent.SetWorldScale3D` (`self.UIMouse1`) (`KismetMathLibrary.MakeVector` _newtrack_0 _newtrack_0 _newtrack_0)))))

(event `self.OnTakeOffMask`
  (`SceneComponent.SetVisibility` (`self.MaskMesh`) false false)
  (goto _label :!via `Reverse`))

(event `self.ReceiveBeginPlay`
  (bind _maskmesh (`self.MaskMesh`))
  (`NiagaraComponent.SetPaused` (`self.InfectionPS`) true)
  (bind _asbp_player_character (cast `/Game/BluePrints/Character/BP_PlayerCharacter` (`GameplayStatics.GetPlayerCharacter` 0)))
  (set `self.PlayerRef` _asbp_player_character)
  (`KismetSystemLibrary.K2_SetTimer` null "FlipFlopIcon" 1.5 true)
  (bind _asbp_game_manager (cast `/Game/BluePrints/Managers/BP_GameManager` (`GameplayStatics.GetGameInstance`)))
  (set `self.GameManagerRef` _asbp_game_manager)
  (`SceneComponent.K2_AttachToComponent` (`self.MaskMesh`) (`self.Mesh`) "head" "KeepWorld" "KeepWorld" "KeepWorld" true)
  (if (`CustomerComponent.HasMask` (`self.CustomerComponent`))
    (`SceneComponent.SetVisibility` _maskmesh true false)
    (else
      (`SceneComponent.SetVisibility` _maskmesh false false)
      (`PrimitiveComponent.SetMaterial` (`self.Mesh`) 0 (`KismetArrayLibrary.Array_Random` (`/Game/BluePrints/Managers/BP_GameManager.M_CustomerSkin` (`self.GameManagerRef`))))
      (bind _output_get (set `self.HairSelection` (`KismetMathLibrary.RandomIntegerInRange` 0 1)))
      (`StaticMeshComponent.SetStaticMesh` (`self.Hair`) (select `int` _output_get :`0` "/Game/Assets/Character/Hair/ShortHair.ShortHair" :`1` "/Game/Assets/Character/Hair/LongHair.LongHair" :!type "StaticMesh Object Reference"))
      (`SceneComponent.K2_AttachToComponent` (`self.Hair`) (`self.Mesh`) "head" "KeepRelative" "KeepRelative" "KeepRelative" true)
      (switch `int` _output_get
        (:`0`
          (`PrimitiveComponent.SetMaterial` (`self.Hair`) 0 (`KismetArrayLibrary.Array_Random` (`/Game/BluePrints/Managers/BP_GameManager.M_LongHairColors` (`self.GameManagerRef`)))))
        (:`1`
          (`PrimitiveComponent.SetMaterial` (`self.Hair`) 0 (`KismetArrayLibrary.Array_Random` (`/Game/BluePrints/Managers/BP_GameManager.M_ShortHairColors` (`self.GameManagerRef`))))))
      (bind _output_get_2 (`self.SetClothes`))
      (switch `int` _output_get_2
        (:`0`
          (`PrimitiveComponent.SetMaterial` (`self.Outfit`) 0 (`KismetArrayLibrary.Array_Random` (`/Game/BluePrints/Managers/BP_GameManager.M_PoloPants0` (`self.GameManagerRef`))))
          (`PrimitiveComponent.SetMaterial` (`self.Outfit`) 1 (`KismetArrayLibrary.Array_Random` (`/Game/BluePrints/Managers/BP_GameManager.M_PoloTop1` (`self.GameManagerRef`)))))
        (:`1`
          (`PrimitiveComponent.SetMaterial` (`self.Outfit`) 0 (`KismetArrayLibrary.Array_Random` (`/Game/BluePrints/Managers/BP_GameManager.M_GirlOutFitSkirt0` (`self.GameManagerRef`))))
          (`PrimitiveComponent.SetMaterial` (`self.Outfit`) 1 (`KismetArrayLibrary.Array_Random` (`/Game/BluePrints/Managers/BP_GameManager.M_GirlOutFitShirt1` (`self.GameManagerRef`))))
          (`PrimitiveComponent.SetMaterial` (`self.Outfit`) 2 (`KismetArrayLibrary.Array_Random` (`/Game/BluePrints/Managers/BP_GameManager.M_GirlOutFitScarf2` (`self.GameManagerRef`)))))
        (:`2`
          (`PrimitiveComponent.SetMaterial` (`self.Outfit`) 0 (`KismetArrayLibrary.Array_Random` (`/Game/BluePrints/Managers/BP_GameManager.M_DungareeDungaree0` (`self.GameManagerRef`))))
          (`PrimitiveComponent.SetMaterial` (`self.Outfit`) 1 (`KismetArrayLibrary.Array_Random` (`/Game/BluePrints/Managers/BP_GameManager.M_DungareeTshirt1` (`self.GameManagerRef`)))))))))

(event `self.OnInfected`
  (params (Cond :type Boolean))
  (`NiagaraComponent.SetPaused` (`self.InfectionPS`) (not Cond))
  (`SceneComponent.SetVisibility` (`self.InfectionPS`) true false))

(event `FlipFlopIcon`
  (bind _uimouse1 (`self.UIMouse1`))
  (bind _uicustomer (`self.UICustomer`))
  (if (> (`/Game/BluePrints/Character/BP_PlayerCharacter.NumberOfCustomersSlapped` (`self.PlayerRef`)) 5)
    (`SceneComponent.SetVisibility` _uicustomer true false :!label _label_2)
    (`SceneComponent.SetVisibility` _uimouse1 false false)
    (else
      (`/Engine/EditorBlueprintResources/StandardMacros.FlipFlop`
        (:`A`
          (`SceneComponent.SetVisibility` _uicustomer false false)
          (`SceneComponent.SetVisibility` _uimouse1 true false))
        (:`B`
          (goto _label_2))))))

(fn `SetClothes`
  (returns (Output_Get :type Integer))
  (locals (ChosenClothes :type Integer :default 0))
  (bind _output_get (set `local.ChosenClothes` (`KismetMathLibrary.RandomIntegerInRange` 0 2)))
  (`SkinnedMeshComponent.SetSkinnedAssetAndUpdate` (`self.Outfit`) (select `int` _output_get :`0` "/Game/Assets/Character/Clothing/CustomerOutfits/PoloOutfit/PoloOutfit.PoloOutfit" :`1` "/Game/Assets/Character/Clothing/CustomerOutfits/GirlOutfit/SchoolOutfit02.SchoolOutfit02" :`2` "/Game/Assets/Character/Clothing/CustomerOutfits/HByxor/HByxorOutfit.HByxorOutfit" :!type "SkeletalMesh Object Reference") true)
  (`SkinnedMeshComponent.SetLeaderPoseComponent` (`self.Outfit`) (`self.Mesh`) false)
  (return _output_get))

(fn `UserConstructionScript`)