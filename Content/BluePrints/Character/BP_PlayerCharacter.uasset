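; Player character that slaps masks on customers, throws them, sprays and sprints, with montages and sounds.
; On BeginPlay it attaches cosmetics, creates the HUD and freezes time until any key press.
; Each tick, the spring-arm camera blends velocity look-ahead with cursor position, easing arm length by cursor distance.
; Timelines scale sprint and throw reminders; after a throw lands, the original customer moves to the landing spot and the thrown stand-in is destroyed.
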(event `Key|E`
  (params (Key :type "Key Structure"))
  ;[1 1 1] Debug for threats
  (:`Pressed`
    (if (not (`self.CooldownSpray`))
      (`GameplayStatics.PlaySoundAtLocation` "/Game/Assets/Sounds/Button_press.Button_press" (`self.K2_GetActorLocation`) (struct) 0.6 (`KismetMathLibrary.RandomFloatInRange` 0.8 1.0) 0.0 "/Game/Assets/Sounds/AttunementTEST.AttunementTEST" "/Game/Assets/Sounds/TEstConcurrency.TEstConcurrency" null)
      (`self.PlayAnimMontage` "/Game/Assets/Character/Anim/ThrowRollStart_Montage.ThrowRollStart_Montage" 5.0)
      (`KismetSystemLibrary.Delay` 0.2)
      (bind _output_get (set `self.CharacterSprayTransform` (`KismetMathLibrary.MakeTransform` (`SceneComponent.K2_GetComponentLocation` (`self.SprayLocation`)) (`self.K2_GetActorRotation`))))
      (bind _returnvalue (`|SpawnActorFromClass` "/Game/BluePrints/Props/BP_InvisibleActor.BP_InvisibleActor_C" _output_get "DontSpawnIfColliding" "OverrideRootScale" null null))
      (`AddComponent|NODE_AddNiagaraComponent-1` :`self` _returnvalue))))

(event `self.ReceiveBeginPlay`
  (`SceneComponent.K2_AttachToComponent` (`self.MaskMesh`) (`self.Mesh`) "head" "KeepWorld" "KeepWorld" "KeepWorld" true)
  (`GameplayStatics.SetGlobalTimeDilation` 0.0)
  (`SkinnedMeshComponent.SetLeaderPoseComponent` (`self.OutFitMesh`) (`self.Mesh`) true)
  (`SceneComponent.K2_AttachToComponent` (`self.Hair`) (`self.Mesh`) "head" "KeepRelative" "KeepRelative" "KeepRelative" true)
  (bind _asbp_game_manager (cast `/Game/BluePrints/Managers/BP_GameManager` (`GameplayStatics.GetGameInstance`)))
  (bind _output_get (set `self.GameManagerRef` _asbp_game_manager))
  (bind _returnvalue (`|CreateWidget` "/Game/BluePrints/UserInterface/UserInterface.UserInterface_C" null _output_get))
  (`UserWidget.AddToViewport` _returnvalue 0)
  (bind _asanim_bp_player (cast `/Game/Assets/Character/Anim/AnimBP_Player` (`SkeletalMeshComponent.GetAnimInstance` (`self.Mesh`))))
  (set `self.AnimBPRef` _asanim_bp_player)
  (`KismetSystemLibrary.Delay` 10.0)
  (`self.SprintReminder`))

(event `Key|Q`
  (params (Key :type "Key Structure"))
  ;[1 1 1] Debug for threats
  (:`Pressed`
    (`GameplayStatics.PlaySoundAtLocation` "/Game/Assets/Sounds/Button_press.Button_press" (`self.K2_GetActorLocation`) (struct) 0.6 (`KismetMathLibrary.RandomFloatInRange` 0.8 1.0) 0.0 "/Game/Assets/Sounds/AttunementTEST.AttunementTEST" "/Game/Assets/Sounds/TEstConcurrency.TEstConcurrency" null)))

(event `Key|AnyKey`
  (params (Key :type "Key Structure"))
  (:`Pressed`
    (`GameplayStatics.SetGlobalTimeDilation` 1.0)))

(event `self.PlayerMaskSlap.OnSlapMask`
  (params (FSlapData :type "SlapData Structure (by ref)"))
  (bind _delay (`self.Delay`))
  (`GameplayStatics.PlaySoundAtLocation` "/Game/Assets/Sounds/Slap_1.Slap_1" (`self.K2_GetActorLocation`) (struct) 0.4 0.75 0.0 "/Game/Assets/Sounds/AttunementTEST.AttunementTEST" "/Game/Assets/Sounds/TEstConcurrency.TEstConcurrency" null)
  (if FSlapData_SlapSucceed
    (`KismetSystemLibrary.PrintString` "Slapped a mask on that customer!" true true (struct :`G` 1.0 :`B` 0.08019 :`A` 1.0))
    (`/Engine/EditorBlueprintResources/StandardMacros.IncrementInt` (`self.NumberOfCustomersSlapped`)
      (:`  `
        _))
    (else
      (`KismetSystemLibrary.PrintString` "That customer already has a mask!" true true (struct :`R` 1.0 :`G` 0.497126 :`B` 0.105561 :`A` 1.0))))
  (set `self.bCanMove` false)
  (`KismetSystemLibrary.PrintString` "Player Slap animation" true true (struct :`G` 0.461277 :`B` 1.0 :`A` 1.0) _delay)
  (`KismetSystemLibrary.Delay` _delay)
  (set `self.bCanMove` true))

(event `Key|Escape` :paused true
  (params (Key :type "Key Structure"))
  ;[1 1 1] Pause Menu
  (:`Pressed`
    (`/Engine/EditorBlueprintResources/StandardMacros.FlipFlop`
      (:`A`
        (bind _returnvalue (`|CreateWidget` "/Game/BluePrints/UserInterface/PauseMenu.PauseMenu_C"))
        (`UserWidget.AddToViewport` _returnvalue 0)
        (`GameplayStatics.SetGamePaused` true))
      (:`B`
        (`Widget.RemoveFromParent` _returnvalue)
        (`GameplayStatics.SetGamePaused` false)))))

(event `Key|LeftShift`
  (params (Key :type "Key Structure"))
  (bind _charactermovement (`self.CharacterMovement`))
  (:`Pressed`
    (set `CharacterMovementComponent.MaxWalkSpeed` 1100.0 _charactermovement :!label _label)
    (set `self.HasSprinted` true)
    (if (`self.ShowingSprintReminder`)
      (bind (_direction _opacity_curve _newtrack_0) (`Timeline|Timeline_0` :!label _label_2)
        (:`Update`
          (`SceneComponent.SetWorldScale3D` (`self.UISprint`) (`KismetMathLibrary.MakeVector` _newtrack_0 _newtrack_0 _newtrack_0))))))
  (:`Released`
    (set `CharacterMovementComponent.MaxWalkSpeed` 700.0 _charactermovement :!label _label_3)))

(event `Key|SpaceBar`
  (params (Key :type "Key Structure"))
  (:`Pressed`
    (goto _label))
  (:`Released`
    (goto _label_3)))

(event `self.ReceiveTick`
  (params (DeltaSeconds :type "Float (single-precision)"))
  (bind _cameramindistance (`self.CameraMinDistance`))
  (bind _cameramaxdistance (`self.CameraMaxDistance`))
  (bind (_cameraseektarget_x _cameraseektarget_y _cameraseektarget_z) (`KismetMathLibrary.BreakVector` (`self.CameraSeekTarget`)))
  (bind _uisprint (`self.UISprint`))
  (bind _returnvalue (`KismetMathLibrary.Vector_Distance` (`self.CameraSeekTarget`) (`self.CursorLocation`)))
  (bind _hitresult (`PlayerController.GetHitResultUnderCursorForObjects` (`GameplayStatics.GetPlayerController` 0) (`|MakeArray` "ObjectTypeQuery5" :!type "EObjectTypeQuery Enum") true))
  (bind (_returnvalue_x _returnvalue_y) (`KismetMathLibrary.BreakVector` (`KismetMathLibrary.VLerp` (`KismetMathLibrary.MakeVector` (- _cameraseektarget_x 500.0) _cameraseektarget_y) (`self.CursorLocation`) (`self.MoveToCursorAlpha`))))
  (set `self.CameraSeekTarget` (`KismetMathLibrary.VInterpTo` (`self.CameraSeekTarget`) (+ (* (`self.GetActorForwardVector`) (* (`self.VelocityLengthMultiplier`) (`KismetMathLibrary.VSize` (`self.GetVelocity`)))) (`self.K2_GetActorLocation`)) (`GameplayStatics.GetWorldDeltaSeconds`) (`self.CameraSeekInterpSpeed`)))
  (if (`GameplayStatics.BreakHitResult` _hitresult)
    (set `self.CursorLocation` (`.Location` (`GameplayStatics.BreakHitResult` _hitresult))))
  (set `self.DesiredArmLength` (+ (`self.BaseLength`) (/ (`|EaseFunction` "ExpoInOut" (`KismetMathLibrary.NormalizeToRange` (`KismetMathLibrary.FClamp` _returnvalue _cameramindistance _cameramaxdistance) _cameramindistance _cameramaxdistance) _returnvalue _cameramaxdistance) (`self.CursorLengthDivider`))))
  (`SceneComponent.K2_SetWorldLocation` (`self.SpringArm`) (`KismetMathLibrary.MakeVector` _returnvalue_x _returnvalue_y (+ _cameraseektarget_z (`self.CameraHeight`))) false false)
  (`SceneComponent.K2_SetWorldRotation` _uisprint (`KismetMathLibrary.FindLookAtRotation` (`SceneComponent.K2_GetComponentLocation` _uisprint) (`self.K2_GetActorLocation` (`PlayerController.PlayerCameraManager` (`GameplayStatics.GetPlayerController` 0)))) false true)
  (`SceneComponent.K2_SetWorldRotation` (`self.UIThrow`) (`KismetMathLibrary.FindLookAtRotation` (`SceneComponent.K2_GetComponentLocation` _uisprint) (`self.K2_GetActorLocation` (`PlayerController.PlayerCameraManager` (`GameplayStatics.GetPlayerController` 0)))) false true)
  (if (not (`KismetMathLibrary.NearlyEqual_FloatFloat` (`self.DesiredArmLength`) (`SpringArmComponent.TargetArmLength` (`self.SpringArm`)) 5.0))
    (set `SpringArmComponent.TargetArmLength` (`KismetMathLibrary.FInterpTo` (`SpringArmComponent.TargetArmLength` (`self.SpringArm`)) (`self.DesiredArmLength`) (`GameplayStatics.GetWorldDeltaSeconds`) (`self.ArmGrowRate`)) (`self.SpringArm`))))

(event `SprintReminder`
  (if (not (`self.HasSprinted`))
    (set `self.ShowingSprintReminder` true)
    (goto _label_2 :!via `ReverseFromEnd`)))

(event `Key|LeftMouseButton`
  (params (Key :type "Key Structure"))
  (:`Pressed`
    (`self.PlayAnimMontage` "/Game/Assets/Character/Anim/Slap_Montage.Slap_Montage")
    (`GameplayStatics.PlaySoundAtLocation` "/Game/Assets/Sounds/Throw_woosh_2.Throw_woosh_2" (`self.K2_GetActorLocation`) (struct) 1.0 (`KismetMathLibrary.RandomFloatInRange` 0.3 0.7) 0.0 "/Game/Assets/Sounds/AttunementTEST.AttunementTEST" "/Game/Assets/Sounds/TEstConcurrency.TEstConcurrency" null)))

(event `Key|RightMouseButton`
  (params (Key :type "Key Structure"))
  (:`Pressed`
    (`self.PlayAnimMontage` "/Game/Assets/Character/Anim/ThrowRollStart_Montage.ThrowRollStart_Montage"))
  (:`Released`
    (`self.PlayAnimMontage` "/Game/Assets/Character/Anim/ThrowRollEnd_Montage.ThrowRollEnd_Montage" 3.0)
    (`GameplayStatics.PlaySoundAtLocation` "/Game/Assets/Sounds/Throw_woosh_1.Throw_woosh_1" (`self.K2_GetActorLocation`) (struct) 0.75 (`KismetMathLibrary.RandomFloatInRange` 0.6 1.0) 0.0 null null null)))

(event `SeeChild`
  (bind _output_get (set `self.ChildrenSeen` (+ (`self.ChildrenSeen`) 1)))
  (`KismetSystemLibrary.PrintString` (`KismetStringLibrary.Conv_IntToString` _output_get)))

(event `self.OnCustomerLanded`
  (params (CustomerAbs :type "AICustomerAbstract Object Reference"))
  (bind _returnvalue (`PlayerGrabComponent.GetOriginalCustomer` (`self.PlayerGrabComponent`)))
  (bind (_returnvalue_x _returnvalue_y _returnvalue_z) (`KismetMathLibrary.BreakVector` (`SceneComponent.K2_GetComponentLocation` (`Character.Mesh` CustomerAbs))))
  (`self.RemoveThrowIndicator`)
  (`PlayerGrabComponent.OnlyRelease` (`self.PlayerGrabComponent`))
  (`GameplayStatics.PlaySoundAtLocation` "/Game/Assets/Sounds/Customer_Scream+impact.Customer_Scream+impact" (`self.K2_GetActorLocation`) (struct) 1.0 (`KismetMathLibrary.RandomFloatInRange` 0.8 1.0) 0.0 "/Game/Assets/Sounds/AttunementTEST.AttunementTEST" "/Game/Assets/Sounds/TEstConcurrency.TEstConcurrency" null)
  (`KismetSystemLibrary.Delay` 2.0)
  (`/Engine/EditorBlueprintResources/StandardMacros.IsValid` CustomerAbs
    (:`Is Valid`
      (if (< _returnvalue_z 100.0)
        (set `self.ZFell` 150.0)
        (else
          (set `self.ZFell` _returnvalue_z)))
      (bind _output_get (set `self.LocationOfLanding` (`KismetMathLibrary.MakeVector` _returnvalue_x _returnvalue_y (`self.ZFell`))))
      (`/Engine/EditorBlueprintResources/StandardMacros.IsValid` _returnvalue
        (:`Is Valid`
          (`self.K2_SetActorLocation` _returnvalue _output_get false true)
          (`PlayerGrabComponent.SetThrowingCustomer` (`self.PlayerGrabComponent`) false)
          (`/Engine/EditorBlueprintResources/StandardMacros.IsValid` CustomerAbs
            (:`Is Valid`
              (`SceneComponent.SetVisibility` (`Actor.RootComponent` CustomerAbs) false true)
              (`KismetSystemLibrary.Delay` 0.05)
              (`self.K2_DestroyActor` CustomerAbs))))
        (:`Is Not Valid`
          (`PlayerGrabComponent.SetThrowingCustomer` (`self.PlayerGrabComponent`) false))))
    (:`Is Not Valid`
      (`PlayerGrabComponent.SetThrowingCustomer` (`self.PlayerGrabComponent`) false))))

(event `RemoveThrowIndicator`
  (bind (_direction _opacity_curve _newtrack_0) (`Timeline|Timeline_1` :!label _label_4)
    (:`Update`
      (`SceneComponent.SetWorldScale3D` (`self.UIThrow`) (`KismetMathLibrary.MakeVector` _newtrack_0 _newtrack_0 _newtrack_0)))))

(event `self.OnGrabSuccess`
  (if (not (`self.HasThrown`))
    (set `self.HasThrown` true)
    (set `self.ShowingThrowReminder` true)
    (goto _label_4 :!via `ReverseFromEnd`)))

(fn `UserConstructionScript`)