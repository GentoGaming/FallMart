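; BP_InfectionCloud is an infection cloud prop that infects any AI customer that begins overlapping it.
; On spawn it destroys other nearby clouds, increments the GameManager's seen-cloud count and raises infection, which is lowered again when the cloud is destroyed.
; Its UIInfectionCloud indicator turns to face the player camera every tick and, after a short delay, animates its scale through a timeline played in reverse.
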(event `self.ReceiveBeginPlay`
  (bind _gamemanagerref (`self.GameManagerRef`))
  (bind _asbp_game_manager (cast `/Game/BluePrints/Managers/BP_GameManager` (`GameplayStatics.GetGameInstance`)))
  (set `self.GameManagerRef` _asbp_game_manager)
  (bind _outactors (`KismetSystemLibrary.SphereOverlapActors` (`self.K2_GetActorLocation`) 30.0 (`|MakeArray` "ObjectTypeQuery2" :!type "EObjectTypeQuery Enum") "BP_InfectionCloud_C" (`|MakeArray` self :!type "Actor Object Reference")))
  (for _array_element _outactors
    (`self.K2_DestroyActor` _array_element))
  (set `/Game/BluePrints/Managers/BP_GameManager.InfectionCloudsSeen` (+ (`/Game/BluePrints/Managers/BP_GameManager.InfectionCloudsSeen` _gamemanagerref) 1) _gamemanagerref)
  (`/Game/BluePrints/Managers/BP_GameManager.ModifyInfection` _gamemanagerref 1)
  (`KismetSystemLibrary.Delay` 1.0)
  (`self.ShowFeedback`))

(event `self.ReceiveDestroyed`
  (bind _gamemanagerref (`self.GameManagerRef`))
  (`/Engine/EditorBlueprintResources/StandardMacros.IsValid` _gamemanagerref
    (:`Is Valid`
      (`/Game/BluePrints/Managers/BP_GameManager.ModifyInfection` _gamemanagerref -1))))

(event `self.ReceiveTick`
  (params (DeltaSeconds :type "Float (single-precision)"))
  (bind _uiinfectioncloud (`self.UIInfectionCloud`))
  (`SceneComponent.K2_SetWorldRotation` _uiinfectioncloud (`KismetMathLibrary.FindLookAtRotation` (`SceneComponent.K2_GetComponentLocation` _uiinfectioncloud) (`self.K2_GetActorLocation` (`PlayerController.PlayerCameraManager` (`GameplayStatics.GetPlayerController` 0)))) false true))

(event `self.ReceiveActorBeginOverlap`
  (params (OtherActor :type "Actor Object Reference"))
  (bind _output_get (set `self.OverlappedActor` OtherActor))
  (bind _asaicustomer_abstract (cast `AICustomerAbstract` _output_get))
  (`CustomerComponent.SetInfected` (`AICustomerAbstract.CustomerComponent` _asaicustomer_abstract) true))

(event `ShowFeedback`
  (bind (_direction _opacity_curve _newtrack_0) (`Timeline|Timeline_0` :!via `ReverseFromEnd`)
    (:`Update`
      (`SceneComponent.SetWorldScale3D` (`self.UIInfectionCloud`) (`KismetMathLibrary.MakeVector` _newtrack_0 _newtrack_0 _newtrack_0)))))

(fn `UserConstructionScript`)