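; BPC_Infection is an actor component that makes its owner a temporary source of infection.
; On BeginPlay it starts a looping SpreadTick timer, with the interval randomized once, that spawns a BP_InfectionCloud at the owner's location and prints a debug message.
; The component destroys itself after a random delay between MinLifespan and MaxLifespan.
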(event `self.ReceiveBeginPlay`
  (`KismetSystemLibrary.K2_SetTimer` null "SpreadTick" (`KismetMathLibrary.RandomFloatInRange` 4.0 7.0) true)
  (`KismetSystemLibrary.Delay` (`KismetMathLibrary.RandomFloatInRange` (`self.MinLifespan`) (`self.MaxLifespan`)))
  (`self.K2_DestroyComponent`))

(event `SpreadTick`
  (`KismetSystemLibrary.PrintString` "Spawn Cloud" true true (struct :`R` 1.0 :`G` 0.084153 :`A` 1.0))
  (`|SpawnActorFromClass` "/Game/BluePrints/Props/BP_InfectionCloud.BP_InfectionCloud_C" (`KismetMathLibrary.MakeTransform` (`Actor.K2_GetActorLocation` (`self.GetOwner`))) "Undefined" "OverrideRootScale" null null))