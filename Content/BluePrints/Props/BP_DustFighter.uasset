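; BP_DustFighter is a prop of a randomly dressed customer character flung around by physics, apparently for a dust-cloud fight.
; Skin, hair and one of three outfits draw random materials from BP_GameManager, with clothing following the body via master pose.
; A physics handle chases a randomly rotating spring arm's end at random intervals, creating erratic motion.
; Timelines animate arm length, revealing the meshes after the intro; PullToCenter reverses one, then destroys the actor.
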(event `self.ReceiveBeginPlay`
  (bind _asbp_game_manager (cast `/Game/BluePrints/Managers/BP_GameManager` (`GameplayStatics.GetGameInstance`)))
  (set `self.GameManagerRef` _asbp_game_manager)
  (`PhysicsHandleComponent.GrabComponentAtLocation` (`self.PhysicsHandle`) (`self.SkeletalMesh`) "None" (`SceneComponent.K2_GetComponentLocation` (`self.ArmEnd`)))
  (set `RotatingMovementComponent.RotationRate` (`KismetMathLibrary.MakeRotator` (`KismetMathLibrary.RandomFloatInRange` 100.0 500.0) (`KismetMathLibrary.RandomFloatInRange` 100.0 500.0) (`KismetMathLibrary.RandomFloatInRange` 100.0 500.0)) (`self.RotatingMovement`))
  (`self.EventSetClothes`)
  (`self.PhysichandleDelayLoopStart`)
  (bind (_direction _newtrack_0) (`Timeline|ModifyArmLength` :!via `PlayFromStart`)
    (:`Update`
      (set `SpringArmComponent.TargetArmLength` _newtrack_0 (`self.SpringArm`)))
    (:`Finished`
      (`SceneComponent.SetVisibility` (`self.SkeletalMesh1`) true true)
      (`SceneComponent.SetVisibility` (`self.SkeletalMesh`) true true))))

(event `PhysichandleDelayLoopStart`
  (`KismetSystemLibrary.Delay` (`KismetMathLibrary.RandomFloatInRange` 0.1 1.5) :!label _label)
  (`PhysicsHandleComponent.SetTargetLocation` (`self.PhysicsHandle`) (`SceneComponent.K2_GetComponentLocation` (`self.ArmEnd`)))
  (goto _label))

(event `EventSetClothes`
  (`PrimitiveComponent.SetMaterial` (`self.SkeletalMesh`) 0 (`KismetArrayLibrary.Array_Random` (`/Game/BluePrints/Managers/BP_GameManager.M_CustomerSkin` (`self.GameManagerRef`))))
  (bind _output_get (set `self.HairSelection` (`KismetMathLibrary.RandomIntegerInRange` 0 1)))
  (`StaticMeshComponent.SetStaticMesh` (`self.HairMesh`) (select `int` _output_get :`0` "/Game/Assets/Character/Hair/ShortHair.ShortHair" :`1` "/Game/Assets/Character/Hair/LongHair.LongHair" :!type "StaticMesh Object Reference"))
  (`SceneComponent.K2_AttachToComponent` (`self.HairMesh`) (`self.SkeletalMesh1`) "head" "KeepRelative" "KeepRelative" "KeepRelative" true)
  (switch `int` _output_get
    (:`0`
      (`PrimitiveComponent.SetMaterial` (`self.HairMesh`) 0 (`KismetArrayLibrary.Array_Random` (`/Game/BluePrints/Managers/BP_GameManager.M_LongHairColors` (`self.GameManagerRef`)))))
    (:`1`
      (`PrimitiveComponent.SetMaterial` (`self.HairMesh`) 0 (`KismetArrayLibrary.Array_Random` (`/Game/BluePrints/Managers/BP_GameManager.M_ShortHairColors` (`self.GameManagerRef`))))))
  (`SceneComponent.K2_AttachToComponent` (`self.MaskMesh`) (`self.SkeletalMesh`) "head" "KeepWorld" "KeepWorld" "KeepWorld" true)
  (`SceneComponent.SetVisibility` (`self.MaskMesh`) true false)
  (bind _output_get_2 (`self.SetClothes`))
  (switch `int` _output_get_2
    (:`0`
      (`PrimitiveComponent.SetMaterial` (`self.SkeletalMesh1`) 0 (`KismetArrayLibrary.Array_Random` (`/Game/BluePrints/Managers/BP_GameManager.M_PoloPants0` (`self.GameManagerRef`))))
      (`PrimitiveComponent.SetMaterial` (`self.SkeletalMesh1`) 1 (`KismetArrayLibrary.Array_Random` (`/Game/BluePrints/Managers/BP_GameManager.M_PoloTop1` (`self.GameManagerRef`)))))
    (:`1`
      (`PrimitiveComponent.SetMaterial` (`self.SkeletalMesh1`) 0 (`KismetArrayLibrary.Array_Random` (`/Game/BluePrints/Managers/BP_GameManager.M_GirlOutFitSkirt0` (`self.GameManagerRef`))))
      (`PrimitiveComponent.SetMaterial` (`self.SkeletalMesh1`) 1 (`KismetArrayLibrary.Array_Random` (`/Game/BluePrints/Managers/BP_GameManager.M_GirlOutFitShirt1` (`self.GameManagerRef`))))
      (`PrimitiveComponent.SetMaterial` (`self.SkeletalMesh1`) 2 (`KismetArrayLibrary.Array_Random` (`/Game/BluePrints/Managers/BP_GameManager.M_GirlOutFitScarf2` (`self.GameManagerRef`)))))
    (:`2`
      (`PrimitiveComponent.SetMaterial` (`self.SkeletalMesh1`) 0 (`KismetArrayLibrary.Array_Random` (`/Game/BluePrints/Managers/BP_GameManager.M_DungareeDungaree0` (`self.GameManagerRef`))))
      (`PrimitiveComponent.SetMaterial` (`self.SkeletalMesh1`) 1 (`KismetArrayLibrary.Array_Random` (`/Game/BluePrints/Managers/BP_GameManager.M_DungareeTshirt1` (`self.GameManagerRef`)))))))

(event `PullToCenter`
  (bind (_direction _newtrack_0) (`Timeline|Timeline_0` :!via `Reverse`)
    (:`Update`
      (set `SpringArmComponent.TargetArmLength` _newtrack_0 (`self.SpringArm`)))
    (:`Finished`
      (`self.K2_DestroyActor`))))

(fn `SetClothes`
  (returns (Output_Get :type Integer))
  (locals (ChosenClothes :type Integer))
  (bind _output_get (set `local.ChosenClothes` (`KismetMathLibrary.RandomIntegerInRange` 0 2)))
  (`SkinnedMeshComponent.SetSkinnedAssetAndUpdate` (`self.SkeletalMesh1`) (select `int` _output_get :`0` "/Game/Assets/Character/Clothing/CustomerOutfits/PoloOutfit/PoloOutfit.PoloOutfit" :`1` "/Game/Assets/Character/Clothing/CustomerOutfits/GirlOutfit/SchoolOutfit02.SchoolOutfit02" :`2` "/Game/Assets/Character/Clothing/CustomerOutfits/HByxor/HByxorOutfit.HByxorOutfit" :!type "SkeletalMesh Object Reference") true)
  (`SkinnedMeshComponent.SetLeaderPoseComponent` (`self.SkeletalMesh1`) (`self.SkeletalMesh`) false)
  (return _output_get))

(fn `UserConstructionScript`)