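; Store item prop whose mesh is either picked at random or set with an optional custom material in the construction script.
; On BeginPlay, an instance without an owner registers with the GameManager and hides its mesh in game.
; An owned instance randomly tilts its mesh, then imitates its owning BP_StoreItem by copying actor scale, mesh and materials.
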(event `self.ReceiveBeginPlay`
  (bind _returnvalue (`self.GetOwner`))
  (bind _staticmeshcomponent (`self.StaticMeshComponent`))
  (`/Engine/EditorBlueprintResources/StandardMacros.IsValid` _returnvalue
    (:`Is Valid`
      (`SceneComponent.K2_SetRelativeRotation` (`self.StaticMeshComponent`) (`KismetMathLibrary.MakeRotator` (`KismetMathLibrary.RandomFloatInRange` -20.0 20.0) (`KismetMathLibrary.RandomFloatInRange` -20.0 20.0) (`KismetMathLibrary.RandomFloatInRange` -20.0 20.0)) false false)
      (bind _asbp_store_item (cast `/Game/BluePrints/Props/BP_StoreItem` _returnvalue))
      (bind _output_get (set `self.ImitationRef` _asbp_store_item))
      (`self.SetActorScale3D` (`self.GetActorScale3D` _output_get))
      (bind _staticmeshcomponent_2 (`StaticMeshActor.StaticMeshComponent` _output_get))
      (`StaticMeshComponent.SetStaticMesh` _staticmeshcomponent (`StaticMeshComponent.StaticMesh` _staticmeshcomponent_2))
      (for (_array_element _array_index) (`MeshComponent.GetMaterials` _staticmeshcomponent_2)
        (`PrimitiveComponent.SetMaterial` _staticmeshcomponent _array_index _array_element)))
    (:`Is Not Valid`
      (bind _asgame_manager (cast `GameManager` (`GameplayStatics.GetGameInstance`)))
      (`GameManager.AddStoreItem` _asgame_manager self)
      (`SceneComponent.SetHiddenInGame` (`self.StaticMeshComponent`) true false))))

(fn `UserConstructionScript`
  (if (`self.UseRandomMesh`)
    (`StaticMeshComponent.SetStaticMesh` (`self.StaticMeshComponent`) (select `int` (`KismetMathLibrary.RandomIntegerInRange` 0 10) :`0` "/Game/Assets/MeatCafeAssets/AssetpCube8.AssetpCube8" :`1` "/Game/Assets/MeatCafeAssets/AssetpCylinder13.AssetpCylinder13" :`2` "/Game/Assets/MeatCafeAssets/AssetpCylinder2.AssetpCylinder2" :`3` "/Game/Assets/MeatCafeAssets/AssetpCylinder3.AssetpCylinder3" :`4` "/Game/Assets/MeatCafeAssets/AssetpCylinder13.AssetpCylinder13" :`5` "/Game/Assets/MeatCafeAssets/AssetpolySurface12.AssetpolySurface12" :`6` "/Game/Assets/MeatCafeAssets/AssetpolySurface13.AssetpolySurface13" :`7` "/Game/Assets/MeatCafeAssets/AssetpolySurface12.AssetpolySurface12" :`8` "/Game/Assets/MeatCafeAssets/AssetpolySurface13.AssetpolySurface13" :`9` "/Game/Assets/MeatCafeAssets/AssetpolySurface14.AssetpolySurface14" :`10` "/Game/Assets/MeatCafeAssets/AssetpolySurface24.AssetpolySurface24" :!type "StaticMesh Object Reference"))
    (else
      (`StaticMeshComponent.SetStaticMesh` (`self.StaticMeshComponent`) (`self.Mesh`))
      (if (`self.UseCustomMaterial`)
        (`PrimitiveComponent.SetMaterial` (`self.StaticMeshComponent`) 0 (`self.CustomMaterial`))))))