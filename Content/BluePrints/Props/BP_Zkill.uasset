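; BP_Zkill is a kill-zone prop that handles actors overlapping it, likely after falling out of the level.
; The player pawn is teleported to the world origin with a fixed rotation instead of being destroyed.
; AI customers are destroyed, and those without a mask first lower threat through the BP_GameManager game instance cached on BeginPlay.
; Any other actor is left untouched.
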(event `self.ReceiveBeginPlay`
  (bind _asbp_game_manager (cast `/Game/BluePrints/Managers/BP_GameManager` (`GameplayStatics.GetGameInstance`)))
  (set `self.GameManagerRef` _asbp_game_manager))

(event `self.ReceiveActorBeginOverlap`
  (params (OtherActor :type "Actor Object Reference"))
  (if (== OtherActor (`GameplayStatics.GetPlayerPawn` 0))
    (`self.K2_SetActorLocationAndRotation` OtherActor (0.0 0.0 0.0) (struct :`Yaw` -180.0) false true)
    (else
      (bind _asaicustomer_abstract (cast `AICustomerAbstract` OtherActor))
      (if (not (`CustomerComponent.HasMask` (`AICustomerAbstract.CustomerComponent` _asaicustomer_abstract)))
        (`/Game/BluePrints/Managers/BP_GameManager.ModifyThreat` (`self.GameManagerRef`) -5.0))
      (`self.K2_DestroyActor` OtherActor))))

(fn `UserConstructionScript`)