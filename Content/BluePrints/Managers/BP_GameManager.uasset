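; Game manager for a store hygiene game: runs a Monday-to-Sunday countdown, hygiene warning bars, money totals and customer spawning, started by BP_GameMode.
; A looping timer raises or lowers hygiene from threat and infection-cloud rates; filled bars only climb, and filling all ends the game.
; When a day's countdown expires, ResetGame fades, clears and respawns actors and sets harder parameters, spawning infection clouds from Wednesday.
; Surviving Sunday shows the win widget.
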(event `self.ReceiveInit`
  (set `self.Today` "D_Monday"))

(event `EventStart`
  (bind _spawning_cool_down (`self.Spawning Cool Down`))
  (bind _returnvalue (`GameplayStatics.GetCurrentLevelName` true))
  (if (not (`KismetStringLibrary.EqualEqual_StrStr` _returnvalue "MainMenuLevel"))
    (`KismetSystemLibrary.K2_SetTimer` null "DayCountdown" (`self.VirtualMinute`) true)
    (set `self.HygienePerBar` (/ (`self.MaxHygieneWarningLevel`) (`KismetMathLibrary.Conv_IntToDouble` (`self.BarIncrements`))))
    (`KismetSystemLibrary.K2_SetTimer` null "HygieneUpdateTick" (`self.HygieneUpdateTickRate`) true)
    (`self.Start Drawing Hud`)
    (bind _outactors (`GameplayStatics.GetAllActorsOfClass` "/Game/BluePrints/Props/BP_StoreItem.BP_StoreItem_C"))
    (for _array_element _outactors
      (`KismetArrayLibrary.Array_Add` (`self.StartingStoreItemsTransform`) (`Actor.GetTransform` _array_element))
      (`KismetArrayLibrary.Array_Add` (`self.StoreItemMeshes`) (`StaticMeshComponent.StaticMesh` (`StaticMeshActor.StaticMeshComponent` _array_element)))
      (`self.ChangeCooldown` _spawning_cool_down)
      (`KismetSystemLibrary.Delay` _spawning_cool_down)
      (`self.BeginSpawnCustomers`))))

(event `HygieneUpdateTick`
  (bind _hygieneupdatetickrate (`self.HygieneUpdateTickRate`))
  (bind _returnvalue (mod (`self.CurrentHygieneWarningLevel`) (`self.HygienePerBar`)))
  (bind _output_get (set `self.IsRising` (> (`self.BuildUpMultiplier`) 0.1)))
  (if _output_get
    (set `self.CurrentHygieneWarningLevel` (+ (`self.CurrentHygieneWarningLevel`) (* (* (* (`self.CurrentBuildUpRate`) (`KismetMathLibrary.SelectFloat` (`self.BuildUpMultiplier`) (* -1 (`self.ReductionRate`)) (`self.IsRising`))) (`self.HygieneUpdateTickRate`)) (`self.TotalHygieneChangeMultiplier`) (`self.CurrentBuildUpRate`) (- 1.0 (* (/ (`self.CurrentHygieneWarningLevel`) (`self.MaxHygieneWarningLevel`)) 0.9)))) :!label _label)
    (if (`self.IsRising`)
      (set `self.AtBarBottomLimit` false)
      (if (>= (`self.CurrentHygieneWarningLevel`) (* (+ (`self.CurrentFilledBars`) 1) (/ (`self.MaxHygieneWarningLevel`) (`KismetMathLibrary.Conv_IntToDouble` (`self.BarIncrements`)))))
        (set `self.CurrentFilledBars` (+ (`self.CurrentFilledBars`) 1))
        (if (>= (`self.CurrentFilledBars`) (`self.BarIncrements`))
          (`self.GameOver`)
          (bind _returnvalue_2 (`|CreateWidget` "/Game/BluePrints/UserInterface/LooseWidgetWindow.LooseWidgetWindow_C"))
          (`UserWidget.AddToViewport` _returnvalue_2 0)
          (`GameplayStatics.SetGamePaused` true)))
      (elif (and (> _returnvalue _hygieneupdatetickrate) (not (`KismetMathLibrary.NearlyEqual_FloatFloat` _returnvalue _hygieneupdatetickrate (`self.ReductionRate`))))
        (set `self.AtBarBottomLimit` false)
        (else
          (set `self.CurrentHygieneWarningLevel` (* (`self.CurrentFilledBars`) (`self.HygienePerBar`)))
          (set `self.AtBarBottomLimit` true))))
    (elif (not (`self.AtBarBottomLimit`))
      (goto _label))))

(event `self.OnThreatChange`
  (params (threatValue :type "Float (single-precision)"))
  (set `self.BuildUpMultiplier` (+ threatValue (`self.BuildUpMultiplier`))))

(event `ModifyThreat`
  (params (Change :type "Float (double-precision)"))
  (set `self.BuildUpMultiplier` (+ Change (`self.BuildUpMultiplier`))))

(event `ModifyCustomerMoney`
  (params (Change :type "Float (double-precision)"))
  ;[1 1 1] Call these with a positive value when you want the store to gain money, and with a negative value for losing money.
  (bind _output_get (set `self.MoneyFromCustomers` (+ Change (`self.MoneyFromCustomers`))))
  (set `self.TotalMoney` (+ _output_get (stale `ModifyBonusMoney` _output_get)) :!label _label_2))

(event `Start Drawing Hud`
  (bind _returnvalue (`GameplayStatics.GetWorldDeltaSeconds`))
  (bind _returnvalue_2 (`GameplayStatics.GetWorldDeltaSeconds`))
  (bind _returnvalue_3 (`GameplayStatics.GetWorldDeltaSeconds`))
  ;[1 1 1] Debug HUD
  (bind _returnvalue_4 (`GameplayStatics.GetCurrentLevelName` true))
  (if (not (`KismetStringLibrary.EqualEqual_StrStr` _returnvalue_4 "MainMenuLevel"))
    (if false :!label _label_3
      (`KismetSystemLibrary.PrintString` (`KismetStringLibrary.Concat_StrStr` "Hygiene Warning Level: " (`KismetStringLibrary.Conv_DoubleToString` (`self.CurrentHygieneWarningLevel`))) true false (struct :`G` 0.66 :`B` 1.0 :`A` 1.0) _returnvalue_2)
      (`KismetSystemLibrary.PrintString` (`KismetStringLibrary.Concat_StrStr` "Filled Bars: " (`KismetStringLibrary.Conv_IntToString` (`self.CurrentFilledBars`))) true false (struct :`R` 0.824505 :`B` 1.0 :`A` 1.0) _returnvalue_2)
      (`KismetSystemLibrary.PrintString` (`KismetStringLibrary.Concat_StrStr` "Is Rising: " (`KismetStringLibrary.Conv_BoolToString` (`self.IsRising`))) true false (struct :`R` 1.0 :`B` 0.021421 :`A` 1.0) _returnvalue_3)
      (`KismetSystemLibrary.PrintString` (`KismetStringLibrary.Concat_StrStr` "At Bar Bottom Limit: " (`KismetStringLibrary.Conv_BoolToString` (`self.AtBarBottomLimit`))) true false (struct :`R` 1.0 :`B` 0.021421 :`A` 1.0) _returnvalue_3)
      (`KismetSystemLibrary.PrintString` (`KismetStringLibrary.Concat_StrStr` "Threat level rising speed: " (`KismetStringLibrary.Conv_DoubleToString` (`self.BuildUpMultiplier`))) true false (struct :`R` 0.876585 :`G` 1.0 :`B` 0.854913 :`A` 1.0) _returnvalue)
      (`KismetSystemLibrary.PrintString` (`KismetStringLibrary.Concat_StrStr` "Cash: " (`KismetStringLibrary.Conv_DoubleToString` (`self.TotalMoney`)) "$") true false (struct :`G` 1.0 :`B` 0.100456 :`A` 1.0) _returnvalue)
      (`KismetSystemLibrary.PrintString` (`KismetStringLibrary.Concat_StrStr` "Infection: " (`KismetStringLibrary.Conv_DoubleToString` (- (`self.CurrentBuildUpRate`) (`self.BaseBuildUpRate`)))) true false (struct :`R` 0.361772 :`G` 0.721873 :`B` 1.0 :`A` 1.0) _returnvalue)
      (`KismetSystemLibrary.PrintString` (`KismetStringLibrary.Concat_StrStr` "Its: " (`|GetEnumeratorNameAsString` (`self.Today`)) "    " (`KismetTextLibrary.Conv_TextToString` (`KismetTextLibrary.Conv_IntToText` (`self.Hours`) false true 2)) ":" (`KismetTextLibrary.Conv_TextToString` (`KismetTextLibrary.Conv_IntToText` (`self.Minutes`) false true 2))) true false (struct :`R` 0.005007 :`G` 0.260417 :`B` 0.007777 :`A` 1.0) _returnvalue)
      (`KismetSystemLibrary.PrintString` (`KismetStringLibrary.Concat_StrStr` (`KismetStringLibrary.Conv_IntToString` (`self.FighterCount`)) " Fighters") true false (struct :`R` 1.0 :`G` 0.853498 :`A` 1.0) (`GameplayStatics.GetWorldDeltaSeconds`))
      (`KismetSystemLibrary.Delay` (* (`GameplayStatics.GetWorldDeltaSeconds`) 0.1))
      (goto _label_3))))

(event `ModifyBonusMoney`
  (params (Change :type "Float (double-precision)"))
  ;[1 1 1] Call these with a positive value when you want the store to gain money, and with a negative value for losing money.
  (bind _output_get (set `self.MoneyFromBonuses` (+ Change (`self.MoneyFromBonuses`))))
  (goto _label_2))

(event `ModifyInfection`
  (params (Change :type Integer))
  (bind _output_get (set `self.InfectionCloudAmount` (+ Change (`self.InfectionCloudAmount`))))
  (set `self.CurrentBuildUpRate` (+ (* _output_get (`self.BuildUpRatePerCloud`)) (`self.BaseBuildUpRate`))))

(event `AddFighter_Event`
  (`/Engine/EditorBlueprintResources/StandardMacros.IncrementInt` (`self.FighterCount`)))

(event `RemoveFighter_Event`
  (`/Engine/EditorBlueprintResources/StandardMacros.DecrementInt` (`self.FighterCount`)))

(event `ResetGame`
  (params (D_Today :type "EDays Enum" :default "D_ChooseADay") (Hours :type Integer) (Minutes :type Integer) (`New Spawnrate` :type "Float (double-precision)"))
  (bind _returnvalue (`|CreateWidget` "/Game/BluePrints/UserInterface/FadeWidget.FadeWidget_C"))
  (bind _fade (`/Game/BluePrints/UserInterface/FadeWidget.Fade` _returnvalue))
  (`UserWidget.PlayAnimation` _returnvalue _fade 0.0 1 "Forward" 1.0 false)
  (`UserWidget.AddToViewport` _returnvalue 0)
  (`KismetSystemLibrary.Delay` (- (`WidgetAnimation.GetEndTime` _fade) 0.1))
  (`KismetSystemLibrary.PrintString` "Day Reset Incoming")
  (set `self.Today` D_Today)
  (`self.SetDay` D_Today)
  (set `self.Hours` Hours)
  (set `self.Minutes` Minutes)
  (`self.ChangeCooldown` `New Spawnrate`)
  (bind _outactors (`GameplayStatics.GetAllActorsOfClass` "/Game/BluePrints/Props/BP_DustFighter.BP_DustFighter_C"))
  (for _array_element _outactors
    (`/Engine/EditorBlueprintResources/StandardMacros.IsValid` _array_element
      (:`Is Valid`
        (`Actor.K2_DestroyActor` _array_element))))
  (set `self.FighterCount` 0)
  (bind _outactors_2 (`GameplayStatics.GetAllActorsOfClass` "/Game/BluePrints/Props/BP_FightCloud.BP_FightCloud_C"))
  (`/Game/BluePrints/Props/BP_FightCloud.CheckScale` (`|GetArrayItem` _outactors_2))
  (bind _outactors_3 (`GameplayStatics.GetAllActorsOfClass` "/Game/BluePrints/Props/BP_InfectionCloud.BP_InfectionCloud_C"))
  (for _array_element_2 _outactors_3
    (`/Engine/EditorBlueprintResources/StandardMacros.IsValid` _array_element_2
      (:`Is Valid`
        (`Actor.K2_DestroyActor` _array_element_2))))
  (bind _outactors_4 (`GameplayStatics.GetAllActorsOfClass` "/Script/Engine.Character"))
  (`KismetArrayLibrary.Array_RemoveItem` _outactors_4 (`GameplayStatics.GetPlayerCharacter` 0))
  (for _array_element_3 _outactors_4
    (`/Engine/EditorBlueprintResources/StandardMacros.IsValid` _array_element_3
      (:`Is Valid`
        (`Actor.K2_DestroyActor` _array_element_3))))
  (bind _outactors_5 (`GameplayStatics.GetAllActorsOfClass` "/Script/Team5_GP3.StoreItem"))
  (for _array_element_4 _outactors_5
    (`/Engine/EditorBlueprintResources/StandardMacros.IsValid` _array_element_4
      (:`Is Valid`
        (`self.RemoveStoreItem` _array_element_4)
        (`Actor.K2_DestroyActor` _array_element_4))))
  (for (_array_element_5 _array_index) (`self.StartingStoreItemsTransform`)
    (bind _returnvalue_2 (`|SpawnActorFromClass` "/Game/BluePrints/Props/BP_StoreItem.BP_StoreItem_C" (`KismetMathLibrary.MakeTransform` (.location _array_element_5) (.rotation _array_element_5)) "Undefined" "OverrideRootScale" null false (`|GetArrayItem` (`self.StoreItemMeshes`) _array_index) null))
    (`self.AddStoreItem` _returnvalue_2))
  (set `self.CurrentFilledBars` 0)
  (set `self.BuildUpMultiplier` 0.0)
  (set `self.InfectionCloudAmount` 0)
  (set `self.CurrentHygieneWarningLevel` 0.0)
  (set `self.IsRising` false)
  (set `self.AtBarBottomLimit` true)
  (`Actor.K2_SetActorLocationAndRotation` (`GameplayStatics.GetPlayerPawn` 0) (0.0 0.0 130.0) (struct :`Yaw` 180.0) false true)
  (bind _returnvalue_3 (`|CreateWidget` "/Game/BluePrints/UserInterface/FadeWidget.FadeWidget_C"))
  (bind _fade_2 (`/Game/BluePrints/UserInterface/FadeWidget.Fade` _returnvalue_3))
  (`UserWidget.PlayAnimation` _returnvalue_3 _fade_2 0.0 1 "Forward" 1.0 false)
  (`UserWidget.AddToViewport` _returnvalue_3 0)
  (`KismetSystemLibrary.Delay` (- (`WidgetAnimation.GetEndTime` _fade_2) (`GameplayStatics.GetWorldDeltaSeconds`)))
  (switch `EDays` (`self.Today`)
    (:`D_Wednesday`
      (`self.SpawnCloud`)
      (set `self.TotalHygieneChangeMultiplier` 0.9))
    (:`D_Thursday`
      (set `self.SpawnCloudCooldown` (- (`self.SpawnCloudCooldown`) 2.0) :!label _label_4)
      (set `self.TotalHygieneChangeMultiplier` (- (`self.TotalHygieneChangeMultiplier`) 0.1)))
    (:`D_Friday`
      (goto _label_4))
    (:`D_Saturday`
      (goto _label_4))
    (:`D_Sunday`
      (goto _label_4))))

(event `SpawnCloud`
  (`KismetSystemLibrary.Delay` (`self.SpawnCloudCooldown`) :!label _label_5)
  (bind _outactors (`GameplayStatics.GetAllActorsOfClass` "/Script/Engine.Character" :!label _label_6))
  (`KismetArrayLibrary.Array_RemoveItem` _outactors (`GameplayStatics.GetPlayerCharacter` 0))
  (bind _outitem (`KismetArrayLibrary.Array_Random` _outactors))
  (`/Engine/EditorBlueprintResources/StandardMacros.IsValid` _outitem
    (:`Is Valid`
      (`|SpawnActorFromClass` "/Game/BluePrints/Props/BP_InfectionCloud.BP_InfectionCloud_C" (`KismetMathLibrary.MakeTransform` (`Actor.K2_GetActorLocation` _outitem)) "Undefined" "OverrideRootScale" null null)
      (goto _label_5))
    (:`Is Not Valid`
      (`KismetSystemLibrary.Delay` 2.0)
      (goto _label_6))))

(fn `Calculate Day Timer`
  (bind _returnvalue (`KismetMathLibrary.Conv_ByteToInt` (`self.Today`)))
  (bind _result (`/Engine/EditorBlueprintResources/StandardMacros.IncrementInt` (`self.Minutes`))
    (:`  `
      (if (> _result 59)
        (`/Engine/EditorBlueprintResources/StandardMacros.IncrementInt` (`self.Hours`)
          (:`  `
            (`self.UIClock` true)
            (set `self.Minutes` 0)
            (if (> (`self.Hours`) 23)
              (if (== _returnvalue (+ (enumcount `EDays`) -1))
                (bind _output_get (set `self.Today` "D_Monday"))
                (else
                  (bind _result_2 (`/Engine/EditorBlueprintResources/StandardMacros.IncrementInt` _returnvalue)
                    (:`  `
                      (set `self.Today` (cast `EDays` (`KismetMathLibrary.Conv_IntToByte` _result_2)))))))
              (`self.SetDay` _output_get))))
        (else
          (`self.UIClock` false))))))

(fn `DayCountdown`
  (bind _result (`/Engine/EditorBlueprintResources/StandardMacros.DecrementInt` (`self.Minutes`))
    (:`  `
      (if (== _result -1)
        (set `self.Minutes` 59)
        (bind _result_2 (`/Engine/EditorBlueprintResources/StandardMacros.DecrementInt` (`self.Hours`))
          (:`  `
            (if (== _result_2 -1)
              (switch `EDays` (`self.Today`)
                (:`D_Monday`
                  (`self.ResetGame` "D_Tuesday" 1 15 4.5))
                (:`D_Tuesday`
                  (`self.ResetGame` "D_Wednesday" 1 30 4.5))
                (:`D_Wednesday`
                  (`self.ResetGame` "D_Thursday" 1 45 4.0))
                (:`D_Thursday`
                  (`self.ResetGame` "D_Friday" 2 0 3.5))
                (:`D_Friday`
                  (`self.ResetGame` "D_Saturday" 2 15 3.0))
                (:`D_Saturday`
                  (`self.ResetGame` "D_Sunday" 2 30 2.5))
                (:`D_Sunday`
                  (bind _returnvalue (`|CreateWidget` "/Game/BluePrints/UserInterface/WinWindowWidget.WinWindowWidget_C"))
                  (`UserWidget.AddToViewport` _returnvalue 0)
                  (`GameplayStatics.SetGamePaused` true))))))))))

(fn `HoursMinutes`)

(fn `UIClock`
  (params (IsHour :type Boolean)))